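; Game mode for a timed card-matching memory game that shows the in-game UI and runs a countdown through a reversed timeline.
; CheckCode uses a FlipFlop to store alternating picks, then compares the two card codes after a short delay.
; A match adds time and score and has BP_Boardgame spawn new cards, while a mismatch deducts time and resets both cards' rotation.
; When time runs out, it opens the game-over level.
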(event Custom|CheckCode
  (params (Code :type Integer) (Actor :type Card%20Base%20BP%20Object%20Reference))
  ;[1 1 1] Guarda los códigos de las cartas en variables locales
  (Variables|Default|SetCode Code)
  (Variables|Default|SetActor Actor)
  (Utilities|FlowControl|FlipFlop
    (:A
      ;;[1 1 1] Primera elección
      (Variables|Default|SetCodeCard1 (Variables|Default|GetCode))
      (Variables|Default|SetCardActor1 (Variables|Default|GetActor)))
    (:B
      ;;[1 1 1] Segunda elección
      (Variables|Default|SetCodeCard2 (Variables|Default|GetCode))
      (Variables|Default|SetCardActor2 (Variables|Default|GetActor))
      (Utilities|FlowControl|Delay 0.2)
      (CallFunction|CheckCardCode))))

(event Custom|CheckCardCode
  ;[1 1 1] Condición que revisa si las cartas son iguales o no
  (if (== (Variables|Default|GetCodeCard1) (Variables|Default|GetCodeCard2))
    (CallFunction|SetNewTime 5.0)
    (CallFunction|Score (Variables|Default|GetAddScore))
    (bind _returnvalue (Actor|GetActorOfClass "/Game/BPs/BP_Boardgame.BP_Boardgame_C"))
    (Utilities|FlowControl|Sequence
      (:then_0
        (Default|SpawnNew _returnvalue (Variables|Default|GetCardActor1)))
      (:then_1
        (Default|SpawnNew2 _returnvalue (Variables|Default|GetCardActor2))))
    (else
      (CallFunction|SetNewTime -1.0)
      (Transformation|SetActorRotation (Variables|Default|GetCardActor1))
      (Transformation|SetActorRotation (Variables|Default|GetCardActor2)))))

(event Custom|SetNewTime
  (params (Time :type Float%20%28single-precision%29))
  ;[1 1 1] Timer
  (bind _output_get (Variables|Default|SetNewTime (+ Time (Variables|Default|GetRemainingTime))))
  (bind _float_counter (Timeline|Timer SetNewTime)
    (:Update
      (bind _output_get_2 (Variables|Default|SetRemainingTime _float_counter))
      (if (<= _output_get_2 0.0)
        (CallFunction|GameOver)))))

(event Custom|Game%20Over
  ;[1 1 1] Game Over
  (Game|OpenLevel(byName) "GameOverScreen"))

(event Custom|Score
  (params (Score :type Integer))
  ;[1 1 1] Score
  (Variables|Default|SetCurrentScore (+ Score (Variables|Default|GetCurrentScore))))

(event EventBeginPlay
  ;[1 1 1] Timer
  (Utilities|FlowControl|Sequence
    (:then_0
      (bind _returnvalue (UserInterface|CreateWidget "/Game/UI/UI_InGame.UI_InGame_C"))
      (UserInterface|Viewport|AddtoViewport _returnvalue 0))
    (:then_1
      (bind _float_counter (Timeline|Timer ReverseFromEnd)
        (:Update
          (bind _output_get (Variables|Default|SetRemainingTime _float_counter))
          (if (<= _output_get 0.0)
            (CallFunction|GameOver)))))))

(fn ConstructionScript)