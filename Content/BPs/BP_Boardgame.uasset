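; Memory-game board Blueprint that spawns the cards, shuffles their layout and resets the game state.
; On BeginPlay it spawns each class from the CardBase_BP actor's CardList at LocationList points, then calls Reset.
; Reset moves randomly picked cards onto those points, then restores score and tries in GM_MemoryGame and clears the draw history.
; GetRandomCard avoids duplicates by re-rolling random indices until one is unused.
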(event Custom|Reset
  ;[1 1 1] Resetea el juego
  (Utilities|FlowControl|Sequence
    (:then_0
      ;;[1 1 1] Ordena las cartas de forma aleatoria
      (for (_ _array_index) (Variables|Default|GetCardActors)
        (bind _randomactor (CallFunction|GetRandomCard))
        (Transformation|SetActorLocationAndRotation _randomactor (Utilities|Array|Get(acopy) (Variables|Default|GetLocationList) _array_index))))
    (:then_1
      ;;[1 1 1] Reset de variables
      (bind _asgm_memory_game (Utilities|Casting|CastToGM_MemoryGame (Game|GetGameMode)))
      (Variables|/Game/GameMode/GM_MemoryGame.GM_MemoryGame_C|SetCurrentScore _asgm_memory_game 0)
      (Variables|/Game/GameMode/GM_MemoryGame.GM_MemoryGame_C|SetTries _asgm_memory_game 10)
      (Variables|Default|SetPreviousIndex -1)
      (Utilities|Array|Clear (Variables|Default|GetIndexList)))))

(event EventBeginPlay
  ;[1 1 1] Inicio del juego
  (bind _returnvalue (Actor|GetActorOfClass "/Game/BPs/CardBase_BP.CardBase_BP_C"))
  (for (_array_element _array_index) (Variables|/Game/BPs/CardBase_BP.CardBase_BP_C|GetCardList _returnvalue)
    (bind _returnvalue_2 (Game|SpawnActorfromClass _array_element (Math|Transform|MakeTransform (Utilities|Array|Get(acopy) (Variables|Default|GetLocationList) _array_index) "0, 0, 0" "1,1,1") "Undefined" 0 0))
    (Utilities|Array|Add (Variables|Default|GetCardActors) _returnvalue_2))
  (CallFunction|Reset))

(fn ConstructionScript)

(fn GetRandomCard
  ;[1 1 1] Nuevo array de cartas con orden aleatorio
  (LocalVariables|SetNewIndex (Math|Random|RandomIntegerinRange 0 (Variables|Default|GetMaxLength)))
  (if (and (!= (LocalVariables|GetNewIndex) (Variables|Default|GetPreviousIndex)) (not (Utilities|Array|ContainsItem (Variables|Default|GetIndexList) (LocalVariables|GetNewIndex)))) :!label _label
    (bind _output_get (Variables|Default|SetPreviousIndex (LocalVariables|GetNewIndex)))
    (Utilities|Array|Add (Variables|Default|GetIndexList) _output_get)
    (return (Utilities|Array|Get(acopy) (Variables|Default|GetCardActors) (Variables|Default|GetPreviousIndex)))
    (else
      (LocalVariables|SetNewIndex (Math|Random|RandomIntegerinRange 0 (Variables|Default|GetMaxLength)))
      (goto _label))))