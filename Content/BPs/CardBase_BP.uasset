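; CardBase_BP is a clickable card actor for a memory game.
; Clicking its collision box raises the cube material's Intensity parameter to highlight the card, then passes the card's CardCode and itself to GM_MemoryGame's CheckCode.
; A ResetColor event sets Intensity back to zero to clear the highlight.
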(event OnClicked(CollisionBox)
  (params (TouchedComponent :type Primitive%20Component%20Object%20Reference) (ButtonPressed :type Key%20Structure :default "None"))
  ;[1 1 1] Cast a GM
  (Rendering|Material|SetScalarParameterValueonMaterials (Variables|Default|GetCube) (Variables|Default|GetIntensity) 1e+01)
  (bind _asgm_memory_game (Utilities|Casting|CastToGM_MemoryGame (Game|GetGameMode)))
  (Default|CheckCode _asgm_memory_game (Variables|CardCode|GetCardCode) self))

(event Custom|ResetColor
  (Rendering|Material|SetScalarParameterValueonMaterials (Variables|Default|GetCube) (Variables|Default|GetIntensity) 0.0))

(fn ConstructionScript)